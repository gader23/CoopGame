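; Grenade projectile actor that explodes on a fixed one-second fuse started at BeginPlay.
; The Explosion event spawns an explosion particle effect and applies radial damage around the actor, credited to the instigator's controller, then destroys the actor.
; A debug sphere drawn after the destroy call visualizes the damage radius.
; Overlap and Tick events are unused, so contact does not trigger detonation in this graph.
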(event `self.ReceiveBeginPlay`
  (`KismetSystemLibrary.Delay` 1.0)
  (`self.Explosion`))

(event `Explosion`
  (bind _returnvalue (`self.K2_GetActorLocation`))
  (bind _damage_radius (`self.Damage Radius`))
  (`GameplayStatics.SpawnEmitterAtLocation` "/Game/WeaponEffects/Explosion/P_Explosion.P_Explosion" _returnvalue)
  (`GameplayStatics.ApplyRadialDamage` :`BaseDamage` 100.0 :`Origin` _returnvalue :`DamageRadius` _damage_radius :`DamageCauser` self :`InstigatedByController` (`self.GetInstigatorController`))
  (`self.K2_DestroyActor`)
  (`KismetSystemLibrary.DrawDebugSphere` _returnvalue _damage_radius 12 (struct :`R` 1.0 :`G` 0.934192 :`A` 1.0) 1.0 2.0))

(fn `UserConstructionScript`)